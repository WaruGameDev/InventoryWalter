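; BP_Item is a pickup actor that adds an item to the player's inventory.
; Its construction script looks up the row selected by ItemDB and applies that row's mesh and name to the static mesh and text render.
; When a BP_ThirdPersonCharacter overlaps the sphere, it passes the row name and Quantity to that character's BPCInventory component, then destroys itself.
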(event `self.Sphere.OnComponentBeginOverlap`
  (params (OverlappedComponent :type "PrimitiveComponent Object Reference") (OtherActor :type "Actor Object Reference") (OtherComp :type "PrimitiveComponent Object Reference") (OtherBodyIndex :type Integer) (bFromSweep :type Boolean) (SweepResult :type "HitResult Structure (by ref)"))
  (bind (_itemdb_datatable _itemdb_rowname) (break `DataTableRowHandle` (`self.ItemDB`)))
  (bind _asbp_third_person_character (cast `/Game/ThirdPerson/Blueprints/BP_ThirdPersonCharacter` OtherActor))
  (`/Game/Blueprint/Component/BPC_Inventory.AddItemToInventory` (`/Game/ThirdPerson/Blueprints/BP_ThirdPersonCharacter.BPC_Inventory` _asbp_third_person_character) _itemdb_rowname (`self.Quantity`))
  (`self.K2_DestroyActor`))

(fn `UserConstructionScript`
  (bind (_itemdb_datatable _itemdb_rowname) (break `DataTableRowHandle` (`self.ItemDB`)))
  (bind _returnvalue (`|GetDataTableRow` _itemdb_datatable _itemdb_rowname)
    (:`then`
      (bind (_nameitem _meshitem) (break `/Game/Blueprint/Data/S_Item` _returnvalue))
      (`StaticMeshComponent.SetStaticMesh` (`self.Item`) _meshitem)
      (`TextRenderComponent.K2_SetText` (`self.TextRender`) (`KismetTextLibrary.Conv_NameToText` _nameitem)))))