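; BP_Door is a door actor that opens by destroying itself once the player has supplied a required quantity of a specific item.
; When BP_ThirdPersonCharacter overlaps its Box, it removes the needed item, identified by data table row name, from the character's inventory component.
; The amount returned is subtracted from the remaining requirement, so partial payments accumulate across overlaps until none is left.
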(event `self.Box.OnComponentBeginOverlap`
  (params (OverlappedComponent :type "PrimitiveComponent Object Reference") (OtherActor :type "Actor Object Reference") (OtherComp :type "PrimitiveComponent Object Reference") (OtherBodyIndex :type Integer) (bFromSweep :type Boolean) (SweepResult :type "HitResult Structure (by ref)"))
  (bind (_itemneeded_datatable _itemneeded_rowname) (break `DataTableRowHandle` (`self.ItemNeeded`)))
  (bind _asbp_third_person_character (cast `/Game/ThirdPerson/Blueprints/BP_ThirdPersonCharacter` OtherActor))
  (bind _itementregados (`/Game/Blueprint/Component/BPC_Inventory.RemoveFromInventory` (`/Game/ThirdPerson/Blueprints/BP_ThirdPersonCharacter.BPC_Inventory` _asbp_third_person_character) _itemneeded_rowname (`self.QuantityNeeded`)))
  (bind _output_get (set `self.QuantityNeeded` (- (`self.QuantityNeeded`) _itementregados)))
  (if (<= _output_get 0)
    (`self.K2_DestroyActor`)))

(fn `UserConstructionScript`)