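; Inventory component that stores items as a map of keys to quantities.
; AddItemToInventory adds the given amount to an existing entry or creates a new one.
; RemoveFromInventory subtracts the requested quantity and deletes the entry when the request uses up or exceeds the stock.
; It returns LastRemove, which updates only when an entry is deleted, so a partial removal returns the previously stored value.
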(fn `AddItemToInventory`
  (params (Key :type "Name (by ref)") (Value :type "Integer (by ref)"))
  (if (`BlueprintMapLibrary.Map_Contains` (`self.Inventory`) Key)
    (`BlueprintMapLibrary.Map_Add` (`self.Inventory`) Key (+ (`BlueprintMapLibrary.Map_Find` (`self.Inventory`) Key) Value))
    (else
      (`BlueprintMapLibrary.Map_Add` (`self.Inventory`) Key Value))))

(fn `RemoveFromInventory`
  (params (ItemName :type "Name (by ref)") (Quantity :type Integer))
  (returns (ItemEntregados :type Integer))
  (bind _value (`BlueprintMapLibrary.Map_Find` (`self.Inventory`) ItemName))
  (bind _value_2 (`BlueprintMapLibrary.Map_Find` (`self.Inventory`) ItemName))
  (bind _returnvalue (- _value Quantity))
  (if (>= _value_2 Quantity)
    (if (> _returnvalue 0)
      (`BlueprintMapLibrary.Map_Add` (`self.Inventory`) (`local.ItemName`) _returnvalue)
      (else
        (bind _output_get (set `self.LastRemove` _value))
        (`BlueprintMapLibrary.Map_Remove` (`self.Inventory`) (`local.ItemName`))))
    (return _output_get)
    (else
      (bind _output_get_2 (set `self.LastRemove` _value_2))
      (`BlueprintMapLibrary.Map_Remove` (`self.Inventory`) (`local.ItemName`))
      (return _output_get_2))))